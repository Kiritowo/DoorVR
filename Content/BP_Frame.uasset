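; BP_Frame is a door frame that swings its Door component while a VR motion controller is inside its Sphere trigger.
; Sphere overlaps with components tagged MotionController set or clear the Hands reference.
; Each tick with a valid Hands calls Rotation, which adds a fixed yaw Step only if the result stays within plus or minus MaxYaw.
; The hand's position does not influence the swing.
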(event OnComponentBeginOverlap(Sphere)
  (params (OverlappedComponent :type Primitive%20Component%20Object%20Reference) (OtherActor :type Actor%20Object%20Reference) (OtherComp :type Primitive%20Component%20Object%20Reference) (OtherBodyIndex :type Integer) (bFromSweep :type Boolean) (SweepResult :type Hit%20Result%20Structure%20%28by%20ref%29))
  (if (Components|ComponentHasTag OtherComp "MotionController")
    (Variables|Default|SetHands OtherComp)))

(event OnComponentEndOverlap(Sphere)
  (params (OverlappedComponent :type Primitive%20Component%20Object%20Reference) (OtherActor :type Actor%20Object%20Reference) (OtherComp :type Primitive%20Component%20Object%20Reference) (OtherBodyIndex :type Integer))
  (if (Components|ComponentHasTag OtherComp "MotionController")
    (Variables|Default|SetHands 0)))

(event EventTick
  (params (DeltaSeconds :type Float%20%28single-precision%29))
  (if (Utilities|IsValid (Variables|Default|GetHands))
    (CallFunction|Rotation)))

(fn ConstructionScript)

(fn Rotation
  (bind _door (Variables|Default|GetDoor))
  (bind _step (Variables|Default|GetStep))
  (bind _maxyaw (Variables|Default|GetMaxYaw))
  (bind _relativerotation (Variables|/Script/Engine.SceneComponent|GetRelativeRotation _door))
  (bind _returnvalue (+ (.yaw _relativerotation) _step))
  (if (not (or (> _returnvalue _maxyaw) (< _returnvalue (* _maxyaw -1.0))))
    (Transformation|AddRelativeRotation _door (Math|Rotator|MakeRotator 0.0 0.0 (Variables|Default|GetStep)) false false)))